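; PolyZone child Blueprint that visualizes the zone's grid, with no active gameplay logic of its own.
; The construction script destroys GridViz's child components, then redraws the grid if PolySpline has more than two points.
; DrawGridData spawns a cell-sized static mesh per grid cell at the actor's height, with material chosen by its within, outside or on-edge flag.
; It also moves an arrow above the grid origin and prints the cell count.
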(fn `Clean`
  (locals (GridChildren :type "Array of SceneComponent Object Reference"))
  (bind _output_get (set `local.GridChildren` (`SceneComponent.GetChildrenComponents` (`self.GridViz`) true)))
  (for _array_element _output_get
    (`/Engine/EditorBlueprintResources/StandardMacros.IsValid` _array_element
      (:`Is Valid`
        (`ActorComponent.K2_DestroyComponent` _array_element)))))

(fn `DrawGridData`
  (bind (_returnvalue_x _returnvalue_y _returnvalue_z) (`KismetMathLibrary.BreakVector` (`self.K2_GetActorLocation`)))
  (bind (_returnvalue_x_2 _returnvalue_y_2 _returnvalue_z_2) (`KismetMathLibrary.BreakVector` (`self.K2_GetActorLocation`)))
  (bind _returnvalue (/ (`self.CellSize`) 100.0))
  (`SceneComponent.K2_SetWorldLocation` (`self.Arrow`) (+ (`self.GridOrigin_WS`) (0.0 0.0 500.0) (`KismetMathLibrary.MakeVector` 0.0 0.0 _returnvalue_z)) false false)
  (bind _returnvalue_2 (`self.GetAllGridCells`))
  (for _array_element _returnvalue_2
    (bind _returnvalue_3 (`self.GetGridCellCenterWorld` _array_element))
    (bind _returnvalue_4 (`AddComponent|NODE_AddStaticMeshComponent-0` :`RelativeTransform` (`KismetMathLibrary.MakeTransform` (0.0 0.0 0.0) (struct) (`KismetMathLibrary.MakeVector` _returnvalue _returnvalue 1.0))))
    (`SceneComponent.K2_SetWorldLocation` _returnvalue_4 (`KismetMathLibrary.MakeVector` (`KismetMathLibrary.BreakVector2D` _returnvalue_3) (`.Y` (`KismetMathLibrary.BreakVector2D` _returnvalue_3)) _returnvalue_z_2) false false)
    (bind _returnvalue_5 (`self.GetGridCellFlag` _array_element))
    (`PrimitiveComponent.SetMaterial` _returnvalue_4 0 (select `PZ_LOOKUP_CELL_FLAGS` _returnvalue_5 :`Within` "/Game/Colors/Green.Green" :`Outside` "/Game/Colors/Red.Red" :`OnEdge` "/Game/Colors/Color_Base.Color_Base" :!type "MaterialInterface Object Reference")))
  (`KismetSystemLibrary.PrintString` (`KismetStringLibrary.Conv_IntToString` (`KismetArrayLibrary.Array_Length` _returnvalue_2))))

(fn `UserConstructionScript`
  (`self.Clean`)
  (if (> (`SplineComponent.GetNumberOfSplinePoints` (`self.PolySpline`)) 2)
    (`self.DrawGridData`)))
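; Junk prop for the PolyZones demo playground that takes on a random shape and reacts to house zones.
; MakeMe runs on construction and BeginPlay, picking a random mesh and world rotation, with an option to exclude chamfer cubes.
; PolyZone enter and exit events cast to Zone_House, turning the mesh solid blue inside and restoring its base material on exit.
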(event `self.ReceiveBeginPlay`
  (`self.MakeMe`))

(event `PolyZone_Interface.EnterPolyZone`
  (params (PolyZone :type "PolyZone Object Reference"))
  (cast `/Game/PolyZones_Demo/Blueprints/Zones/Zone_House` PolyZone)
  (`PrimitiveComponent.SetMaterial` (`self.Mesh`) 0 "/Game/PolyZones_Demo/Materials/Colors/MI_Solid_Blue.MI_Solid_Blue"))

(event `PolyZone_Interface.ExitPolyZone`
  (params (PolyZone :type "PolyZone Object Reference"))
  (cast `/Game/PolyZones_Demo/Blueprints/Zones/Zone_House` PolyZone)
  (`PrimitiveComponent.SetMaterial` (`self.Mesh`) 0 "/Game/PolyZones_Demo/Materials/Colors/Color_Base.Color_Base"))

(fn `MakeMe`
  (bind _mesh (`self.Mesh`))
  (if (`self.NoBoxes`)
    (`KismetArrayLibrary.Array_RemoveItem` (`self.Meshes`) "/Game/PolyZones_Demo/LevelPrototyping/Meshes/SM_ChamferCube.SM_ChamferCube"))
  (`StaticMeshComponent.SetStaticMesh` _mesh (`KismetArrayLibrary.Array_Random` (`self.Meshes`)))
  (`SceneComponent.K2_SetWorldRotation` _mesh (`KismetMathLibrary.RandomRotator` true) false false))

(fn `UserConstructionScript`
  (`self.MakeMe`))
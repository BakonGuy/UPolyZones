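; Star_Actor is a playground prop in the PolyZones demo that celebrates a finish with an animated star.
; On BeginPlay it caches every Star_Cube actor in the level.
; StartStarAnim sets the finish text, switches the star to a gold material and plays a timeline that lerps it between start and end transforms.
; Each timeline update wakes the cubes' rigid bodies so the moving star does not clip through them.
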(event `self.ReceiveBeginPlay`
  (bind _outactors (`GameplayStatics.GetAllActorsOfClass` "/Game/PolyZones_Demo/Blueprints/PlaygroundProps/Star_Cube.Star_Cube_C"))
  (set `self.Cubes` _outactors))

(event `StartStarAnim`
  (bind (_starttransform_location _starttransform_rotation) (`KismetMathLibrary.BreakTransform` (`self.StartTransform`)))
  (bind (_endtransform_location _endtransform_rotation) (`KismetMathLibrary.BreakTransform` (`self.EndTransform`)))
  (`TextRenderComponent.K2_SetText` (`self.TextRender`) (`self.FinishText`))
  (`PrimitiveComponent.SetMaterial` (`self.Star`) 0 "/Game/PolyZones_Demo/Materials/Star/Star_Gold.Star_Gold")
  (bind (_direction _lerppos _lerprot) (`Timeline|AnimateStar`)
    (:`Update`
      (`SceneComponent.K2_SetRelativeLocationAndRotation` (`self.Star`) (`KismetMathLibrary.VLerp` _starttransform_location _endtransform_location _lerppos) (`KismetMathLibrary.RLerp` _starttransform_rotation _endtransform_rotation _lerprot true) false false)
      ;[1 1 1] Make sure we are not clipping
      (for _array_element (`self.Cubes`)
        (`PrimitiveComponent.WakeRigidBody` (`/Game/PolyZones_Demo/Blueprints/PlaygroundProps/Star_Cube.SM_ChamferCube` _array_element) "None")))))

(fn `UserConstructionScript`)
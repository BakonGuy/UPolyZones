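; PolyZone_DemoPlayer is the PolyZones demo's player controller, managing the on-screen UI for cashier and ATM interactions.
; On BeginPlay, the local controller creates a Demo_UI widget, adds it to the viewport and keeps a reference.
; ShowCashierUI and ShowATM_UI forward visibility to that widget and call ShowCursor, which toggles the mouse cursor and switches between Game-and-UI and Game-Only input modes.
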(event `self.ReceiveBeginPlay`
  (if (`self.IsLocalPlayerController`)
    (bind _returnvalue (`|CreateWidget` "/Game/PolyZones_Demo/Blueprints/UI/Demo_UI.Demo_UI_C" self))
    (`UserWidget.AddToViewport` _returnvalue 0)
    (set `self.DemoUI` _returnvalue)))

(event `ShowCashierUI`
  (params (Show :type Boolean))
  (`/Game/PolyZones_Demo/Blueprints/UI/Demo_UI.ShowCashierUI` (`self.DemoUI`) Show)
  (`self.ShowCursor` Show))

(event `ShowATM_UI`
  (params (Show :type Boolean))
  (`/Game/PolyZones_Demo/Blueprints/UI/Demo_UI.ShowATM_UI` (`self.DemoUI`) Show)
  (`self.ShowCursor` Show))

(event `ShowCursor`
  (params (Show :type Boolean))
  (bind _output_get (set `self.bShowMouseCursor` Show))
  (if _output_get
    (`WidgetBlueprintLibrary.SetInputMode_GameAndUIEx` self null)
    (else
      (`WidgetBlueprintLibrary.SetInputMode_GameOnly` self))))

(fn `UserConstructionScript`)
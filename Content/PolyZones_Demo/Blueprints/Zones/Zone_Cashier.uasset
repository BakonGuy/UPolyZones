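; Demo cashier zone Blueprint from PolyZones_Demo that reports when the third-person character enters or leaves it.
; The poly zone enter and exit events filter actors by casting to BP_ThirdPersonCharacter.
; Each then prints the character's display name with an entered or exited message on screen, tinted by the zone's color and kept out of the log.
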(event `self.OnEnterPolyZone`
  (params (EnteredActor :type "Actor Object Reference"))
  (bind _asbp_third_person_character (cast `/Game/PolyZones_Demo/Blueprints/BP_ThirdPersonCharacter` EnteredActor))
  (`KismetSystemLibrary.PrintString` (`KismetStringLibrary.Concat_StrStr` (`KismetSystemLibrary.GetDisplayName` _asbp_third_person_character) " Entered Cashier Zone") true false (`KismetMathLibrary.Conv_ColorToLinearColor` (`self.ZoneColor`))))

(event `self.OnExitPolyZone`
  (params (ExitedActor :type "Actor Object Reference"))
  (bind _asbp_third_person_character (cast `/Game/PolyZones_Demo/Blueprints/BP_ThirdPersonCharacter` ExitedActor))
  (`KismetSystemLibrary.PrintString` (`KismetStringLibrary.Concat_StrStr` (`KismetSystemLibrary.GetDisplayName` _asbp_third_person_character) " Exited Cashier Zone") true false (`KismetMathLibrary.Conv_ColorToLinearColor` (`self.ZoneColor`))))

(fn `UserConstructionScript`)
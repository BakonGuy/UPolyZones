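; Demo PolyZone for a house cleanup task that rewards the player once all junk has been moved out of the zone.
; Junk entering or leaving updates a world text count of zone actors minus the player pawn, with sound cues; the enter sound is muted briefly after level load.
; An exit that empties the zone triggers the win: DudeText thanks the player, the demo UI grants life savings and the zone destroys itself.
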(event `self.ReceiveBeginPlay`
  ;[1 1 1] Prevent sounds on level load
  (`KismetSystemLibrary.Delay` 1.0)
  (set `self.PlaySounds` true)
  (`KismetSystemLibrary.LoadAsset_Blocking` "/Game/PolyZones_Demo/Sounds/Ping.Ping"))

(event `self.OnEnterPolyZone`
  (params (EnteredActor :type "Actor Object Reference"))
  (cast `/Game/PolyZones_Demo/Blueprints/PlaygroundProps/Junk` EnteredActor)
  (`self.UpdateJunkCount`)
  (if (`self.PlaySounds`)
    (`GameplayStatics.PlaySound2D` "/Game/PolyZones_Demo/Sounds/NoMoney.NoMoney" 1.0 1.0 0.0 null null)))

(event `self.OnExitPolyZone`
  (params (ExitedActor :type "Actor Object Reference"))
  (cast `/Game/PolyZones_Demo/Blueprints/PlaygroundProps/Junk` ExitedActor)
  (`self.UpdateJunkCount`)
  (`GameplayStatics.PlaySound2D` "/Game/PolyZones_Demo/Sounds/Ping.Ping" 1.0 1.0 0.0 null null)
  (`self.CheckForWin`))

(fn `CheckForWin`
  (bind _returnvalue (`self.GetAllActorsInPolyZone`))
  (`KismetArrayLibrary.Array_RemoveItem` _returnvalue (`GameplayStatics.GetPlayerPawn` 0))
  (if (<= (`KismetArrayLibrary.Array_Length` _returnvalue) 0)
    (`GameplayStatics.PlaySound2D` "/Game/PolyZones_Demo/Sounds/GoldStar.GoldStar" 1.0 1.0 0.0 null null)
    (bind _dudetext (`self.DudeText`)
      (:`then`
        (bind _textrender (`TextRenderActor.TextRender` _dudetext))
        (`TextRenderComponent.K2_SetText` _textrender (`KismetTextLibrary.Conv_StringToText` "Wow, it's never been so clean! \nHere have my life savings! \nJust think of all the boxes you can buy now!"))
        (`TextRenderComponent.SetTextRenderColor` _textrender (`self.Green`))
        (`self.GiveLifeSavings`)
        (`self.K2_DestroyActor`))
      (:`else`))))

(fn `GiveLifeSavings`
  (bind _aspoly_zone_demo_player (cast `/Game/PolyZones_Demo/Blueprints/PolyZone_DemoPlayer` (`GameplayStatics.GetPlayerController` 0)))
  (`/Game/PolyZones_Demo/Blueprints/UI/Demo_UI.GiveLifeSavings` (`/Game/PolyZones_Demo/Blueprints/PolyZone_DemoPlayer.DemoUI` _aspoly_zone_demo_player)))

(fn `UpdateJunkCount`
  (bind _junkcounttext (`self.JunkCountText`)
    (:`then`
      (bind _returnvalue (`self.GetAllActorsInPolyZone`))
      (`KismetArrayLibrary.Array_RemoveItem` _returnvalue (`GameplayStatics.GetPlayerPawn` 0))
      (`TextRenderComponent.K2_SetText` (`TextRenderActor.TextRender` _junkcounttext) (`KismetTextLibrary.Conv_StringToText` (`KismetStringLibrary.Concat_StrStr` "Junk in House: " (`KismetStringLibrary.Conv_IntToString` (`KismetArrayLibrary.Array_Length` _returnvalue))))))
    (:`else`)))

(fn `UserConstructionScript`)
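; Demo PolyZone that tracks Star_Cube objects brought into it to trigger a star animation.
; Entering cubes and any exit update the StarActor's stacked number from the count of all actors in the zone.
; When a cube entry brings that count to five or more, it starts the star animation and the zone destroys itself.
; Junk actors that enter are destroyed.
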(event `self.OnEnterPolyZone`
  (params (EnteredActor :type "Actor Object Reference"))
  (cast `/Game/PolyZones_Demo/Blueprints/PlaygroundProps/Star_Cube` EnteredActor
    (:`then`
      (`self.UpdateStar`)
      (bind _staractor (`self.StarActor`)
        (:`then`
          ;[1 1 1] Wait until no objects in zone
          (bind _returnvalue (`self.GetAllActorsInPolyZone`))
          (if (>= (`KismetArrayLibrary.Array_Length` _returnvalue) 5)
            (`/Game/PolyZones_Demo/Blueprints/PlaygroundProps/Star_Actor.StartStarAnim` _staractor)
            (`self.K2_DestroyActor`)))
        (:`else`)))
    (:`CastFailed`
      (bind _asjunk (cast `/Game/PolyZones_Demo/Blueprints/PlaygroundProps/Junk` EnteredActor))
      (`self.K2_DestroyActor` _asjunk))))

(event `self.OnExitPolyZone`
  (params (ExitedActor :type "Actor Object Reference"))
  (`self.UpdateStar`))

(event `UpdateStar`
  (bind _staractor (`self.StarActor`)
    (:`then`
      (bind _returnvalue (`self.GetAllActorsInPolyZone`))
      (`/Game/PolyZones_Demo/Blueprints/PlaygroundProps/Star_Actor.SetStackedNum` _staractor (`KismetArrayLibrary.Array_Length` _returnvalue)))
    (:`else`)))

(fn `UserConstructionScript`)
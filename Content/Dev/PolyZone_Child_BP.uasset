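; Dev child Blueprint of a PolyZone actor for visualizing and profiling its spline polygon and grid containment queries.
; On PolyZoneConstructed it draws the spline bounds and, when ShowDebugGrid is set, spawns a mesh per grid cell colored Outside, Within or OnEdge.
; Test functions time point-in-polygon, grid-flag and PolyZone checks at random locations, printing results and drawing debug spheres.
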(event `TestCells`
  (bind _returnvalue (`self.GetAllGridCells`))
  (`KismetSystemLibrary.PrintString` (`KismetStringLibrary.Concat_StrStr` "Grid Cells Manual: " (`KismetStringLibrary.Conv_IntToString` (`KismetArrayLibrary.Array_Length` _returnvalue))) true true (struct :`R` 1.0 :`G` 0.771999 :`A` 1.0) 10.0))

(event `self.PolyZoneConstructed`
  (`self.Construct`))

(fn `Construct`
  (bind (_origin _boxextent) (`KismetSystemLibrary.GetComponentBounds` (`self.PolySpline`)))
  (bind _returnvalue (`SplineComponent.GetNumberOfSplinePoints` (`self.PolySpline`)))
  (`KismetSystemLibrary.PrintString` (`KismetStringLibrary.Concat_StrStr` (`KismetStringLibrary.Conv_IntToString` _returnvalue) " PolyZone points") true true (struct :`R` 1.0 :`B` 0.837406 :`A` 1.0) 10.0)
  (if (> _returnvalue 2)
    (`KismetSystemLibrary.DrawDebugBox` _origin _boxextent (struct :`R` 0.282604 :`B` 0.302083 :`A` 1.0) (struct) 5.0 50.0)
    (if (`self.ShowDebugGrid`)
      (`self.DrawGridData`))))

(fn `DrawGridData`
  (bind (_returnvalue_x _returnvalue_y _returnvalue_z) (`KismetMathLibrary.BreakVector` (`self.K2_GetActorLocation`)))
  (bind (_returnvalue_x_2 _returnvalue_y_2 _returnvalue_z_2) (`KismetMathLibrary.BreakVector` (`self.K2_GetActorLocation`)))
  (bind _returnvalue (/ (`self.CellSize`) 100.0))
  (`SceneComponent.K2_SetWorldLocation` (`self.Arrow`) (+ (`self.GridOrigin_WS`) (0.0 0.0 500.0) (`KismetMathLibrary.MakeVector` 0.0 0.0 _returnvalue_z)) false false)
  (bind _returnvalue_2 (`self.GetAllGridCells`))
  (for _array_element _returnvalue_2
    (bind _returnvalue_3 (`self.GetGridCellCenterWorld` _array_element))
    (bind _returnvalue_4 (`AddComponent|NODE_AddStaticMeshComponent-0` :`RelativeTransform` (`KismetMathLibrary.MakeTransform` (0.0 0.0 0.0) (struct) (`KismetMathLibrary.MakeVector` _returnvalue _returnvalue 1.0))))
    (`SceneComponent.K2_SetWorldLocation` _returnvalue_4 (`KismetMathLibrary.MakeVector` (.x _returnvalue_3) (.y _returnvalue_3) _returnvalue_z_2) false false)
    (bind _returnvalue_5 (`self.GetGridCellFlag` _array_element))
    (`PrimitiveComponent.SetMaterial` _returnvalue_4 0 (select `POLYZONE_CELL_FLAGS` _returnvalue_5 :`Outside` "/Game/Dev/Colors/Red.Red" :`Within` "/Game/Dev/Colors/Green.Green" :`OnEdge` "/Game/Dev/Colors/Color_Base.Color_Base" :!type "MaterialInterface Object Reference")))
  (`KismetSystemLibrary.PrintString` (`KismetStringLibrary.Concat_StrStr` "Grid Cells: " (`KismetStringLibrary.Conv_IntToString` (`KismetArrayLibrary.Array_Length` _returnvalue_2))) true true (struct :`R` 1.0 :`G` 0.771999 :`A` 1.0) 10.0))

(fn `PrintCells`
  (bind _returnvalue (`self.GetAllGridCells`))
  (`KismetSystemLibrary.PrintString` (`KismetStringLibrary.Conv_IntToString` (`KismetArrayLibrary.Array_Length` _returnvalue)) true true (struct :`R` 1.0 :`A` 1.0)))

(fn `Test_Grid_Algo`
  (locals (RandomLocation :type "Vector Structure") (StartTime :type "Float (double-precision)" :default 0.0) (EndTime :type "Float (double-precision)" :default 0.0))
  (bind (_randomlocation_x _randomlocation_y) (`KismetMathLibrary.BreakVector` (`local.RandomLocation`)))
  (bind _output_get (set `local.RandomLocation` (* (`KismetMathLibrary.RandomUnitVector`) (`self.RandomVectorRange`))))
  (bind _returnvalue (`PerformanceTool.GetCurrentTimeMs`))
  (set `local.StartTime` _returnvalue)
  (bind _returnvalue_2 (`self.GetFlagAtLocation` _output_get))
  (bind _returnvalue_3 (`PerformanceTool.GetCurrentTimeMs`))
  (set `local.EndTime` _returnvalue_3)
  (`KismetSystemLibrary.PrintString` (`KismetStringLibrary.Concat_StrStr` (`KismetStringLibrary.Conv_DoubleToString` (* (- (`local.EndTime`) (`local.StartTime`)) 1000.0)) " ms" " - Flag: " (`|GetEnumeratorNameAsString` _returnvalue_2)))
  (`KismetSystemLibrary.DrawDebugSphere` (`KismetMathLibrary.MakeVector` _randomlocation_x _randomlocation_y 400.0) 100.0 12 (struct :`R` 1.0 :`G` 1.0 :`B` 1.0 :`A` 1.0) 2.0 10.0))

(fn `Test_PIP_Algo`
  (locals (RandomLocation :type "Vector Structure") (StartTime :type "Float (double-precision)" :default 0.0) (EndTime :type "Float (double-precision)" :default 0.0))
  (bind _returnvalue (* (`KismetMathLibrary.RandomUnitVector`) (`self.RandomVectorRange`)))
  (set `local.RandomLocation` _returnvalue)
  (bind _returnvalue_2 (`PerformanceTool.GetCurrentTimeMs`))
  (set `local.StartTime` _returnvalue_2)
  (bind _returnvalue_3 (`self.IsPointWithinPolygon` (`KismetMathLibrary.Conv_VectorToVector2D` _returnvalue)))
  (bind _returnvalue_4 (`PerformanceTool.GetCurrentTimeMs`))
  (set `local.EndTime` _returnvalue_4)
  (`KismetSystemLibrary.PrintString` (`KismetStringLibrary.Concat_StrStr` (`KismetStringLibrary.Conv_DoubleToString` (* (- (`local.EndTime`) (`local.StartTime`)) 1000.0)) " ms" " - Within: " (`KismetStringLibrary.Conv_BoolToString` _returnvalue_3)))
  (`KismetSystemLibrary.DrawDebugSphere` (`local.RandomLocation`) 1000.0 12 (struct :`R` 1.0 :`G` 1.0 :`B` 1.0 :`A` 1.0) 2.0 50.0))

(fn `Test_PZ_Algo`
  (locals (RandomLocation :type "Vector Structure") (StartTime :type "Float (double-precision)" :default 0.0) (EndTime :type "Float (double-precision)" :default 0.0))
  (bind (_returnvalue_x _returnvalue_y _returnvalue_z) (`KismetMathLibrary.BreakVector` (`self.K2_GetActorLocation`)))
  (bind (_randomlocation_x _randomlocation_y) (`KismetMathLibrary.BreakVector` (`local.RandomLocation`)))
  (bind _output_get (set `local.RandomLocation` (* (`KismetMathLibrary.RandomUnitVector`) (`self.RandomVectorRange`))))
  (bind _returnvalue (`PerformanceTool.GetCurrentTimeMs`))
  (set `local.StartTime` _returnvalue)
  (bind _returnvalue_2 (`self.IsPointWithinPolyZone` (`KismetMathLibrary.MakeVector` (.x _output_get) (.y _output_get) (+ _returnvalue_z 10.0))))
  (bind _returnvalue_3 (`PerformanceTool.GetCurrentTimeMs`))
  (set `local.EndTime` _returnvalue_3)
  (`KismetSystemLibrary.PrintString` (`KismetStringLibrary.Concat_StrStr` (`KismetStringLibrary.Conv_DoubleToString` (* (- (`local.EndTime`) (`local.StartTime`)) 1000.0)) " ms" " - Within: " (`KismetStringLibrary.Conv_BoolToString` _returnvalue_2)))
  (`KismetSystemLibrary.FlushPersistentDebugLines`)
  (`KismetSystemLibrary.DrawDebugSphere` (`KismetMathLibrary.MakeVector` _randomlocation_x _randomlocation_y 400.0) 100.0 12 (struct :`R` 1.0 :`B` 0.841436 :`A` 1.0) 2.0 10.0))

(fn `UserConstructionScript`
  (`parent.UserConstructionScript`))